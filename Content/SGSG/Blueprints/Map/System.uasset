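; Star system node on the galaxy map that procedurally generates its star, planets and moons and opens system view when clicked.
; GenerateSystem uses the MapManager's random stream for names, sizes and orbits, typing stars and planets by size via data tables.
; MakeConnections grows RangeBox to find neighbors, then randomly links them with two-way JumpLanes, using temporary JumpLaneChecker actors to reject overlapping lanes.
; Empire home systems get magenta names and a connection bias.
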(event `SetSystemName`
  (params (NewName :type String))
  (bind _output_get (set `self.SystemName` NewName))
  (`TextRenderComponent.K2_SetText` (`self.Name`) (`KismetTextLibrary.Conv_StringToText` _output_get)))

(event `SetEmpireHomeSystem`
  (set `self.ConnectionBias` 2.0)
  (`TextRenderComponent.SetTextRenderColor` (`self.Name`) (make `Color` 255 0 255 255)))

(event `PrepSystemGeneration`
  (`SceneComponent.SetRelativeScale3D` (`self.RangeBox`) (0.5 0.5 0.5)))

(event `MakeConnections`
  (bind _overlappingactors (`self.GetOverlappingActors` "System_C"))
  (bind _returnvalue (`self.K2_GetActorLocation`))
  (bind _manager (`self.Manager`))
  (bind _range (`self.Range`))
  ;[1 1 1] ensuring we have enough sytems to connect to
  (while (< (`KismetArrayLibrary.Array_Length` _overlappingactors) 4)
    (`SceneComponent.SetRelativeScale3D` (`self.RangeBox`) (`KismetMathLibrary.MakeVector` _range _range _range))
    (set `self.Range` (+ (`self.Range`) 0.1)))
  (for _array_element _overlappingactors
    ;[1 1 1] Will it connect to the system?
    (bind _assystem (cast `/Game/SGSG/Blueprints/Map/System` _array_element))
    (if (and (> (* (`KismetMathLibrary.RandomFloatInRangeFromStream` (`/Game/SGSG/Blueprints/Management/MapManager.RandomStream` _manager) 0.0 5.0) (`/Game/SGSG/Blueprints/Management/MapManager.StarlaneFrequency` _manager) (`self.ConnectionBias`)) 1.0) (not (`KismetArrayLibrary.Array_Contains` (`self.ConnectedSystems`) _assystem)))
      (bind _returnvalue_2 (`self.K2_GetActorLocation` _assystem))
      (bind _returnvalue_3 (`|SpawnActorFromClass` "/Game/SGSG/Blueprints/Map/JumpLaneChecker.JumpLaneChecker_C" (`KismetMathLibrary.MakeTransform` (`KismetMathLibrary.MakeVector` (/ (+ (.x _returnvalue_2) (.x _returnvalue)) 2.0) (/ (+ (.y _returnvalue_2) (.y _returnvalue)) 2.0) (/ (+ (.z _returnvalue_2) (.z _returnvalue)) 2.0)) (`KismetMathLibrary.FindLookAtRotation` _returnvalue_2 _returnvalue) (`KismetMathLibrary.MakeVector` 1.0 1.0 (- (/ (`KismetMathLibrary.Sqrt` (+ (`KismetMathLibrary.Square` (- (.x _returnvalue_2) (.x _returnvalue))) (`KismetMathLibrary.Square` (- (.y _returnvalue_2) (.y _returnvalue))) (`KismetMathLibrary.Square` (- (.z _returnvalue_2) (.z _returnvalue))))) 100.0) 0.4))) "AlwaysSpawn" "MultiplyWithRoot" null null))
      (if (not (> (+ (`KismetArrayLibrary.Array_Length` (`self.GetOverlappingActors` _returnvalue_3 "System_C")) (`KismetArrayLibrary.Array_Length` (`self.GetOverlappingActors` _returnvalue_3 "/Game/SGSG/Blueprints/Map/JumpLane.JumpLane_C"))) 2))
        (bind _returnvalue_4 (`|SpawnActorFromClass` "/Game/SGSG/Blueprints/Map/JumpLane.JumpLane_C" (`self.GetTransform` _returnvalue_3) "AlwaysSpawn" "MultiplyWithRoot" null null))
        (`self.ConnectToSystem` self _assystem _returnvalue_4)
        (`self.ConnectToSystem` _assystem self _returnvalue_4))
      (`self.K2_DestroyActor` _returnvalue_3)))
  ;[1 1 1] after connections
  (`SceneComponent.SetRelativeScale3D` (`self.RangeBox`) (0.5 0.5 0.5))
  (if (<= (`KismetArrayLibrary.Array_Length` (`self.ConnectedSystems`)) 0)
    (`self.MakeConnections`)))

(event `self.ReceiveActorBeginCursorOver`
  (`SceneComponent.SetVisibility` (`self.RangeBox`) true false))

(event `self.ReceiveActorEndCursorOver`
  (`SceneComponent.SetVisibility` (`self.RangeBox`) false false))

(event `self.ReceiveActorOnClicked`
  (params (ButtonPressed :type "Key Structure"))
  (bind _asp_map (cast `/Game/SGSG/Blueprints/Character/P_Map` (`GameplayStatics.GetPlayerCharacter` 0)))
  (`/Game/SGSG/Blueprints/Character/P_Map.EnterSystemView` _asp_map self))

(event `ConnectToSystem`
  (params (OtherSystem :type "/Game/SGSG/Blueprints/Map/System Object Reference") (JumpLane :type "/Game/SGSG/Blueprints/Map/JumpLane Object Reference"))
  (`KismetArrayLibrary.Array_Add` (`self.ConnectedSystems`) OtherSystem)
  (`KismetArrayLibrary.Array_Add` (`self.JumpLanes`) JumpLane))

(event `self.ReceiveBeginPlay`
  (bind _outactors (`GameplayStatics.GetAllActorsOfClass` "/Game/SGSG/Blueprints/Management/MapManager.MapManager_C"))
  (for _array_element _outactors
    (set `self.Manager` _array_element))
  (`SceneComponent.SetVisibility` (`self.RangeBox`) false false))

(event `GenerateSystem`
  (bind _currentdistance (`self.CurrentDistance`))
  (bind _size_left (`self.Size Left`))
  (bind _systemname (`self.SystemName`))
  (bind _currentdistance_2 (`self.CurrentDistance`))
  (bind _randomstream (`/Game/SGSG/Blueprints/Management/MapManager.RandomStream` (`self.Manager`)))
  (if (`KismetStringLibrary.IsEmpty` _systemname)
    (`self.SetSystemName` (`KismetStringLibrary.Concat_StrStr` (`KismetArrayLibrary.Array_RandomFromStream` (`|MakeArray` "Kepler" "Sagan" "Hubble" "Galilei" "Tyson" "Copernicus" "Brahe" "Huygens" "Herschel" "Laplace" "Eratosthenes" "Aryabhata" "Bhāskara" "Aristarchus" "Halley") _randomstream) (`KismetStringLibrary.Concat_StrStr` "-" (`KismetStringLibrary.Conv_IntToString` (`KismetMathLibrary.RandomIntegerInRangeFromStream` _randomstream 100 999))))))
  (bind _output_get (set `self.SystemInfo` (make `/Game/SGSG/Data/structs/S_SystemInfo` (make `/Game/SGSG/Data/structs/S_StarInfo` _systemname (`|MakeArray`) (`KismetArrayLibrary.Array_RandomFromStream` (`|MakeArray` (`KismetMathLibrary.RandomFloatInRangeFromStream` _randomstream 0.1 0.9) (`KismetMathLibrary.RandomFloatInRangeFromStream` _randomstream 0.7 0.9) (`KismetMathLibrary.RandomFloatInRangeFromStream` _randomstream 0.7 1.1) (`KismetMathLibrary.RandomFloatInRangeFromStream` _randomstream 0.7 1.5) (`KismetMathLibrary.RandomFloatInRangeFromStream` _randomstream 0.7 3.0) (`KismetMathLibrary.RandomFloatInRangeFromStream` _randomstream 0.1 0.9) (`KismetMathLibrary.RandomFloatInRangeFromStream` _randomstream 0.7 0.9) (`KismetMathLibrary.RandomFloatInRangeFromStream` _randomstream 0.7 1.1) (`KismetMathLibrary.RandomFloatInRangeFromStream` _randomstream 0.7 1.5) (`KismetMathLibrary.RandomFloatInRangeFromStream` _randomstream 0.1 0.9) (`KismetMathLibrary.RandomFloatInRangeFromStream` _randomstream 0.7 0.9) (`KismetMathLibrary.RandomFloatInRangeFromStream` _randomstream 0.7 1.1) (`KismetMathLibrary.RandomFloatInRangeFromStream` _randomstream 0.7 6.0) (`KismetMathLibrary.RandomFloatInRangeFromStream` _randomstream 0.7 15.0)) _randomstream)) "UNNAMED")))
  (set `self.PlanetNumber` 0)
  (bind (_starname _satelites _size) (break `/Game/SGSG/Data/structs/S_StarInfo` (`.CentralStar_27_F4F518E54FBA95CE173E76BCCFC1466E` (break `/Game/SGSG/Data/structs/S_SystemInfo` _output_get))))
  (bind _type (`self.GetStarTypeBasedOnSize` _size))
  (bind _output_get_2 (set `self.SystemInfo` (make `/Game/SGSG/Data/structs/S_SystemInfo` (make `/Game/SGSG/Data/structs/S_StarInfo` _starname _satelites _size _type) _starname)))
  (`|ExecutionSequence`
    (:`then_0`
      (bind _returnvalue (* (`KismetMathLibrary.Sqrt` _size) 0.1))
      (`SceneComponent.SetRelativeScale3D` (`self.Star`) (`KismetMathLibrary.MakeVector` _returnvalue _returnvalue _returnvalue))
      (`PrimitiveComponent.SetMaterial` (`self.Star`) 0 (`BlueprintMapLibrary.Map_Find` (`self.StarMaterialMap`) _type)))
    (:`then_1`
      (bind (_starname_2 _satelites_2 _size_2) (break `/Game/SGSG/Data/structs/S_StarInfo` (`.CentralStar_27_F4F518E54FBA95CE173E76BCCFC1466E` (break `/Game/SGSG/Data/structs/S_SystemInfo` _output_get_2))))
      (bind _returnvalue_2 (* _size_2 0.15))
      (set `self.CurrentDistance` _returnvalue_2)
      (bind _returnvalue_3 (* _size_2 30.0))
      (set `self.Size Left` (* _returnvalue_3 1.1))
      (while (and (>= (`self.Size Left`) _returnvalue_3) (<= (`self.PlanetNumber`) (* _returnvalue_3 2.0)) (<= (+ (`self.CurrentDistance`) 0.1) (* _size_2 40.0)))
        (bind _result (`/Engine/EditorBlueprintResources/StandardMacros.IncrementInt` (`self.PlanetNumber`))
          (:`  `
            (bind _output_get_3 (set `self.CurrentDistance` (`KismetMathLibrary.RandomFloatInRangeFromStream` _randomstream (+ _currentdistance 0.5) (`KismetMathLibrary.FMin` (+ _currentdistance 1.0) (* _returnvalue_2 40.0)))))
            (bind _returnvalue_4 (`KismetArrayLibrary.Array_Add` _satelites_2 (make `/Game/SGSG/Data/structs/S_PlanetInfo` (`KismetStringLibrary.Concat_StrStr` _starname_2 (`KismetStringLibrary.Concat_StrStr` "-" (`KismetStringLibrary.Conv_IntToString` _result))) (`|MakeArray`) _output_get_3 (`KismetArrayLibrary.Array_RandomFromStream` (`|MakeArray` (`KismetMathLibrary.RandomFloatInRangeFromStream` _randomstream 0.1 13.0) (`KismetMathLibrary.RandomFloatInRangeFromStream` _randomstream 0.1 10.0) (`KismetMathLibrary.RandomFloatInRangeFromStream` _randomstream 0.1 7.0) (`KismetMathLibrary.RandomFloatInRangeFromStream` _randomstream 0.1 4.0) (`KismetMathLibrary.RandomFloatInRangeFromStream` _randomstream 0.1 1.0) (`KismetMathLibrary.RandomFloatInRangeFromStream` _randomstream 0.1 7.0) (`KismetMathLibrary.RandomFloatInRangeFromStream` _randomstream 0.1 4.0) (`KismetMathLibrary.RandomFloatInRangeFromStream` _randomstream 0.1 1.0)) _randomstream))))
            (bind (_bodyname _moons _orbitaldistance _bodysize) (break `/Game/SGSG/Data/structs/S_PlanetInfo` (`|GetArrayItem` _satelites_2 _returnvalue_4)))
            (set `self.Size Left` (- (`self.Size Left`) _bodysize))
            (bind _type_2 (`self.GetPlanetTypeFromSize` _bodysize))
            (`KismetArrayLibrary.Array_Set` _satelites_2 _returnvalue_4 (make `/Game/SGSG/Data/structs/S_PlanetInfo` _bodyname _moons _orbitaldistance _bodysize _type_2 (`KismetArrayLibrary.Array_RandomFromStream` (`|MakeArray` "NewEnumerator4" "NewEnumerator3" "NewEnumerator2" "NewEnumerator1" "NewEnumerator0" :!type "/Game/SGSG/Data/Enums/RockyTypes Enum") _randomstream))))))
      (for (_array_element _array_index) (`.Satelites_19_B7F65B8F4854372B8BE6A8866FE9492F` (break `/Game/SGSG/Data/structs/S_StarInfo` (`.CentralStar_27_F4F518E54FBA95CE173E76BCCFC1466E` (break `/Game/SGSG/Data/structs/S_SystemInfo` (`self.SystemInfo`)))))
        (`KismetArrayLibrary.Array_Clear` (`self.MoonArray`))
        (bind (_bodyname_2 _moons_2 _orbitaldistance_2 _bodysize_2) (break `/Game/SGSG/Data/structs/S_PlanetInfo` _array_element))
        (if (>= _bodysize_2 1.0)
          (set `self.PlanetNumber` 0)
          (set `self.CurrentDistance` 0.1)
          (bind _returnvalue_5 (/ (/ _bodysize_2 10.0) 10.0))
          (set `self.Size Left` _returnvalue_5)
          (while (>= (`self.Size Left`) (/ _returnvalue_5 2.0))
            (`/Engine/EditorBlueprintResources/StandardMacros.IncrementInt` (`self.PlanetNumber`)
              (:`  `
                (bind _s_mooninfo (make `/Game/SGSG/Data/structs/S_MoonInfo` (`KismetStringLibrary.Concat_StrStr` _bodyname_2 (`KismetStringLibrary.Concat_StrStr` "-" (`KismetStringLibrary.Conv_IntToString` (`self.PlanetNumber`)))) (`KismetMathLibrary.RandomFloatInRangeFromStream` _randomstream (+ _currentdistance_2 0.05) (+ _currentdistance_2 0.1)) (`KismetArrayLibrary.Array_RandomFromStream` (`|MakeArray` (`KismetMathLibrary.RandomFloatInRangeFromStream` _randomstream 0.005 (`KismetMathLibrary.FMin` _size_left 1.0)) (`KismetMathLibrary.RandomFloatInRangeFromStream` _randomstream 0.005 (`KismetMathLibrary.FMin` (/ _size_left 2.0) 1.0)) (`KismetMathLibrary.RandomFloatInRangeFromStream` _randomstream 0.005 0.02) :!type "Float (double-precision)") _randomstream) "NewEnumerator0" (`KismetArrayLibrary.Array_RandomFromStream` (`|MakeArray` "NewEnumerator4" "NewEnumerator3" "NewEnumerator2" "NewEnumerator1" "NewEnumerator0" :!type "/Game/SGSG/Data/Enums/RockyTypes Enum") _randomstream)))
                (`KismetArrayLibrary.Array_Add` (`self.MoonArray`) _s_mooninfo)
                (bind (_bodyname_3 _orbitaldistance_3 _bodysize_3) (break `/Game/SGSG/Data/structs/S_MoonInfo` _s_mooninfo))
                (set `self.Size Left` (- (`self.Size Left`) _bodysize_3))
                (set `self.CurrentDistance` _orbitaldistance_3))))
          (bind (_bodyname_4 _moons_3 _orbitaldistance_4 _bodysize_4 _bodytype _rockytype) (break `/Game/SGSG/Data/structs/S_PlanetInfo` _array_element))
          (`KismetArrayLibrary.Array_Set` (`.Satelites_19_B7F65B8F4854372B8BE6A8866FE9492F` (break `/Game/SGSG/Data/structs/S_StarInfo` (`.CentralStar_27_F4F518E54FBA95CE173E76BCCFC1466E` (break `/Game/SGSG/Data/structs/S_SystemInfo` (`self.SystemInfo`))))) _array_index (make `/Game/SGSG/Data/structs/S_PlanetInfo` _bodyname_4 (`self.MoonArray`) _orbitaldistance_4 _bodysize_4 _bodytype _rockytype)))))))

(fn `GetPlanetTypeFromSize`
  (params (Size :type "Float (double-precision)"))
  (returns (Type :type "/Game/SGSG/Data/Enums/E_PlanetSizes Enum"))
  (locals (PlanetSizeType :type "/Game/SGSG/Data/Enums/E_PlanetSizes Enum"))
  (bind _outrownames (`DataTableFunctionLibrary.GetDataTableRowNames` "/Game/SGSG/Data/Tables/PlanetTypesFixed.PlanetTypesFixed"))
  (for _array_element _outrownames
    (bind _returnvalue (`|GetDataTableRow` "/Game/SGSG/Data/Tables/PlanetTypesFixed.PlanetTypesFixed" _array_element)
      (:`then`
        (bind (_min _max _size) (break `/Game/SGSG/Data/structs/S_PlanetSizeInfoFixed` _returnvalue))
        (if (and (<= _min Size) (>= _max Size))
          (set `local.PlanetSizeType` _size)))))
  (return (`local.PlanetSizeType`)))

(fn `GetStarTypeBasedOnSize`
  (params (Size :type "Float (double-precision)"))
  (returns (Type :type "/Game/SGSG/Data/Enums/E_StarSizes Enum"))
  (locals (StarSizeType :type "/Game/SGSG/Data/Enums/E_StarSizes Enum"))
  (bind _outrownames (`DataTableFunctionLibrary.GetDataTableRowNames` "/Game/SGSG/Data/Tables/StarTypes.StarTypes"))
  (for _array_element _outrownames
    (bind _returnvalue (`|GetDataTableRow` "/Game/SGSG/Data/Tables/StarTypes.StarTypes" _array_element)
      (:`then`
        (bind (_min _max _type) (break `/Game/SGSG/Data/structs/S_StarSizeTypes` _returnvalue))
        (if (and (<= _min Size) (>= _max Size))
          (set `local.StarSizeType` _type)))))
  (return (`local.StarSizeType`)))

(fn `UserConstructionScript`)