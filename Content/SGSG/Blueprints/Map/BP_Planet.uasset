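; BP_Planet is a map planet actor that displays its name on a text plaque.
; SetName sets the plaque text, then offsets it along negative X by a distance based on the square root of the sphere's scale.
; It also sets the name source's relative yaw to the negated actor yaw, cancelling the planet's rotation for the label.
; The construction script is empty.
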(event `SetName`
  (params (Name :type String))
  (bind _nameplaque (`self.NamePlaque`))
  (`TextRenderComponent.K2_SetText` _nameplaque (`KismetTextLibrary.Conv_StringToText` Name))
  (`SceneComponent.K2_SetRelativeLocation` _nameplaque (`KismetMathLibrary.MakeVector` (- -50.0 (* (`KismetMathLibrary.Sqrt` (.x (`SceneComponent.RelativeScale3D` (`self.Sphere`)))) 100.0)) 0.0 10.0) false false)
  (`SceneComponent.K2_SetRelativeRotation` (`self.NameSource`) (`KismetMathLibrary.MakeRotator` 0.0 0.0 (.yaw (`KismetMathLibrary.NegateRotator` (`self.K2_GetActorRotation`)))) false false))

(fn `UserConstructionScript`)