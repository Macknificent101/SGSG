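; Map manager that procedurally generates a galaxy of star systems from a seeded random stream, using the current time for seed zero.
; A looping timer scatters systems in a flat ring, rejects overlaps and widens the ring after repeated failures.
; It then picks random empire homes and generates each system and its connections on chained timers, reporting progress to MenuUi.
; Finally, it gives P_Map the galaxy bounds and loads the last system.
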(event `CancelGeneration`
  (if (`KismetSystemLibrary.K2_IsValidTimerHandle` (stale `GenerateGalaxy` _returnvalue_2))
    (`KismetSystemLibrary.K2_ClearAndInvalidateTimerHandle` (stale `GenerateGalaxy` _returnvalue_2)))
  (if (`KismetSystemLibrary.K2_IsValidTimerHandle` (stale `FinalizeGalaxy` _returnvalue))
    (`KismetSystemLibrary.K2_ClearAndInvalidateTimerHandle` (stale `FinalizeGalaxy` _returnvalue))))

(event `GenerateGalaxy`
  (bind _galaxysize (`self.GalaxySize`))
  (bind _returnvalue (* (`KismetMathLibrary.MultiplyByPi` (`KismetMathLibrary.Sqrt` (`KismetMathLibrary.Conv_IntToDouble` _galaxysize))) 7.5))
  ;[1 1 1] this sets up initial parameters based off the galaxy size
  (set `self.RemainingSystemsToGenerate` _galaxysize)
  (set `self.CenterSize` _returnvalue)
  (set `self.GalaxyEdge` (* _returnvalue 2.0))
  (bind _returnvalue_2 (`KismetSystemLibrary.K2_SetTimerDelegate` (delegate `Make System`) 0.001 true))
  (set `self.EmpireCount` (/ (`self.GalaxySize`) 33)))

(event `Make System`
  (bind _randomstream (`self.RandomStream`))
  (bind _galaxyedge (`self.GalaxyEdge`))
  (bind _centersize (`self.CenterSize`))
  (bind _returnvalue (* _galaxyedge -1.0))
  (bind _returnvalue_2 (`KismetMathLibrary.FMin` (/ (`self.GalaxySize`) 10) 25.0))
  ;[1 1 1] If all the systems have been generated, it's time to move to the next stage
  (if (> (`self.RemainingSystemsToGenerate`) 0)
    ;[1 1 1] When there are too many system spawn rejects, that means there is likely not enough space. so, add more space.
    ;
    ; however, if this happens too many times, it's possible there is something wrong, so it will end the loop immediately and go on to the next stage of gen
    (if (>= (`self.SystemSpawnFailures`) (`self.GalaxySize`))
      (set `self.GalaxyEdge` (+ (`self.GalaxyEdge`) (* (`self.CenterSize`) 0.1)))
      (set `self.SystemSpawnFailures` 0)
      (if (>= (`self.GalaxyEdge`) (* (`self.CenterSize`) 2.0))
        (set `self.CenterSize` (+ _centersize (* _centersize 0.5))))
      (else
        ;[1 1 1] This all finds a valid location to attempt to spawn a new system
        (bind _output_get (set `self.TempPosition` (`KismetMathLibrary.MakeVector` (`KismetMathLibrary.RandomFloatInRangeFromStream` _randomstream _returnvalue _galaxyedge) (`KismetMathLibrary.RandomFloatInRangeFromStream` _randomstream _returnvalue _galaxyedge) (`KismetMathLibrary.RandomFloatInRangeFromStream` _randomstream (* _returnvalue_2 -1.0) _returnvalue_2))))
        (bind _returnvalue_3 (`KismetMathLibrary.Vector_Distance` _output_get (`self.K2_GetActorLocation`)))
        (if (and (>= _returnvalue_3 (`self.CenterSize`)) (<= _returnvalue_3 (`self.GalaxyEdge`)))
          ;[1 1 1] This determines if the system spawn needs to get rejected. if the system overlaps another system, they are too cl;ose together, so the spawn must be rejected.
          (bind _returnvalue_4 (`|SpawnActorFromClass` "/Game/SGSG/Blueprints/Map/System.System_C" (`KismetMathLibrary.MakeTransform` _output_get) "Undefined" "MultiplyWithRoot" null null))
          (if (> (`KismetArrayLibrary.Array_Length` (`self.GetOverlappingActors` _returnvalue_4 "/Game/SGSG/Blueprints/Map/System.System_C")) 0)
            (`self.K2_DestroyActor` _returnvalue_4)
            (`/Engine/EditorBlueprintResources/StandardMacros.IncrementInt` (`self.SystemSpawnFailures`))
            (else
              (bind _returnvalue_5 (`KismetArrayLibrary.Array_Add` (`self.Systems`) _returnvalue_4))
              (set `/Game/SGSG/Blueprints/Map/System.SystemID` _returnvalue_5 _returnvalue_4)
              (`/Engine/EditorBlueprintResources/StandardMacros.DecrementInt` (`self.RemainingSystemsToGenerate`)
                (:`  `
                  (bind _foundwidgets (`WidgetBlueprintLibrary.GetAllWidgetsOfClass` "/Game/SGSG/Blueprints/UI/MenuUi.MenuUi_C"))
                  (for _array_element _foundwidgets
                    (`/Game/SGSG/Blueprints/UI/MenuUi.UpdateProgess` _array_element 1)))))))))
    (else
      (`KismetSystemLibrary.K2_ClearAndInvalidateTimerHandle` (stale `GenerateGalaxy` _returnvalue_2))
      (`self.FinalizeGalaxy`))))

(event `FinalizeGalaxy`
  ;[1 1 1] this sets up some important info for systems to keep track of
  (for _ (range (+ (`self.EmpireCount`) 1))
    (`/Game/SGSG/Blueprints/Map/System.SetEmpireHomeSystem` (`KismetArrayLibrary.Array_RandomFromStream` (`self.Systems`) (`self.RandomStream`))))
  ;[1 1 1] this means it's time to generate another system
  (bind _returnvalue (`KismetSystemLibrary.K2_SetTimerDelegate` (delegate `GenerateSystem`) 0.005 :!label _label)))

(event `SystemGenerated`
  ;[1 1 1] this means it's time to generate another system
  (`/Engine/EditorBlueprintResources/StandardMacros.IncrementInt` (`self.CurrentSystem`)
    (:`  `
      (goto _label))))

(event `GenerateSystem`
  (bind _systems (`self.Systems`))
  (bind _systems_2 (`self.Systems`))
  (bind _currentsystem (`self.CurrentSystem`))
  (bind _output (`|GetArrayItem` _systems_2 _currentsystem))
  ;[1 1 1] this calls all needed events to generate a system, then says to go generate another one. if all of them have been generated, it's time to finish gen by telling the player character their bounds.
  (if (>= (- (`KismetArrayLibrary.Array_Length` _systems_2) 1) _currentsystem)
    (`/Game/SGSG/Blueprints/Map/System.PrepSystemGeneration` _output)
    (`/Game/SGSG/Blueprints/Map/System.MakeConnections` _output)
    (`/Game/SGSG/Blueprints/Map/System.GenerateSystem` _output)
    (`self.SystemGenerated`)
    (bind _foundwidgets (`WidgetBlueprintLibrary.GetAllWidgetsOfClass` "/Game/SGSG/Blueprints/UI/MenuUi.MenuUi_C"))
    (for _array_element _foundwidgets
      (`/Game/SGSG/Blueprints/UI/MenuUi.UpdateProgess` _array_element 2))
    (else
      (bind _outactors (`GameplayStatics.GetAllActorsOfClass` "/Game/SGSG/Blueprints/Character/P_Map.P_Map_C"))
      (for _array_element_2 _outactors
        (set `/Game/SGSG/Blueprints/Character/P_Map.Bounds` (`self.GalaxyEdge`) _array_element_2)
        (`/Game/SGSG/Blueprints/Character/P_Map.LoadSystem` _array_element_2 (`|GetArrayItem` _systems (`KismetArrayLibrary.Array_LastIndex` _systems))))
      (`KismetSystemLibrary.K2_ClearAndInvalidateTimerHandle` (stale `FinalizeGalaxy` _returnvalue)))))

(event `SetSeed`
  (params (Seed :type Integer))
  (bind _randomstream (`self.RandomStream`))
  (`KismetMathLibrary.ResetRandomStream` _randomstream)
  (if (== Seed 0)
    (bind _output_get (set `self.Seed` (`KismetMathLibrary.Conv_Int64ToInt` (`KismetMathLibrary.ToUnixTimestamp` (`KismetMathLibrary.Now`)))))
    (`KismetMathLibrary.SetRandomStreamSeed` _randomstream _output_get)
    (bind _foundwidgets (`WidgetBlueprintLibrary.GetAllWidgetsOfClass` "/Game/SGSG/Blueprints/UI/MenuUi.MenuUi_C"))
    (for _array_element _foundwidgets
      (`EditableTextBox.SetText` (`/Game/SGSG/Blueprints/UI/MenuUi.GalaxySeed` _array_element) (`KismetTextLibrary.Conv_IntToText` (`self.Seed`))))
    (else
      (bind _output_get_2 (set `self.Seed` Seed))
      (`KismetMathLibrary.SetRandomStreamSeed` _randomstream _output_get_2))))

(fn `UserConstructionScript`)