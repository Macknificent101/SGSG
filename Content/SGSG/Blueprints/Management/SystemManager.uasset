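; SystemManager builds the visual layout of a star system from a SystemInfo structure, replacing any previously loaded one.
; LoadSystem clears the old actors, then names, scales and skins the central star using square-root size and type-to-material maps.
; For each satellite and its moons, it spawns a BP_Planet at a randomized position scaled by orbital distance, plus a plane mesh with an orbit material.
; Spawned planets, moons and orbit planes are tracked in arrays that ClearSystem destroys.
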(event `LoadSystem`
  (params (`System Info` :type "/Game/SGSG/Data/structs/S_SystemInfo Structure"))
  (bind _star (`self.Star`))
  (bind _name (`self.Name`))
  (bind (_starname _satelites _size _type) (break `/Game/SGSG/Data/structs/S_StarInfo` (`.CentralStar_27_F4F518E54FBA95CE173E76BCCFC1466E` (break `/Game/SGSG/Data/structs/S_SystemInfo` `System Info`))))
  (bind _returnvalue (`KismetMathLibrary.MultiplyByPi` (`KismetMathLibrary.RandomFloatInRange` 0.0 2.0)))
  (bind _returnvalue_2 (`KismetMathLibrary.MultiplyByPi` (`KismetMathLibrary.RandomFloatInRange` 0.0 2.0)))
  (bind _returnvalue_3 (* (`KismetMathLibrary.Sqrt` _size) 5.0))
  (`|ExecutionSequence`
    (:`then_0`
      (`self.ClearSystem`))
    (:`then_1`
      (`TextRenderComponent.K2_SetText` _name (`KismetTextLibrary.Conv_StringToText` _starname))
      (`SceneComponent.SetRelativeScale3D` _star (`KismetMathLibrary.MakeVector` _returnvalue_3 _returnvalue_3 _returnvalue_3))
      (`SceneComponent.K2_SetRelativeLocation` _name (`KismetMathLibrary.MakeVector` (+ (* _returnvalue_3 -100.0) -100.0)) false false)
      (`PrimitiveComponent.SetMaterial` _star 0 (`BlueprintMapLibrary.Map_Find` (`self.StarTypeMap`) _type))
      (for (_array_element _array_index) _satelites
        (bind (_bodyname _moons _orbitaldistance _bodysize _bodytype _rockytype) (break `/Game/SGSG/Data/structs/S_PlanetInfo` _array_element))
        (bind _returnvalue_4 (+ (* _orbitaldistance 50.0) 0.1))
        (bind _returnvalue_5 (`|SpawnActorFromClass` "/Script/Engine.StaticMeshActor" (`KismetMathLibrary.MakeTransform` (`self.K2_GetActorLocation`) (struct) (`KismetMathLibrary.MakeVector` _returnvalue_4 _returnvalue_4 _returnvalue_4)) "Undefined" "MultiplyWithRoot" null null))
        (`StaticMeshActor.SetMobility` _returnvalue_5 "Stationary")
        (bind _staticmeshcomponent (`StaticMeshActor.StaticMeshComponent` _returnvalue_5))
        (`StaticMeshComponent.SetStaticMesh` _staticmeshcomponent "/Engine/BasicShapes/Plane.Plane")
        (`PrimitiveComponent.SetMaterial` _staticmeshcomponent 0 "/Game/SGSG/Materials/materials/M_Orbit.M_Orbit")
        (`PrimitiveComponent.SetCollisionProfileName` _staticmeshcomponent "NoCollision" true)
        (`KismetArrayLibrary.Array_Add` (`self.Orbitals`) _returnvalue_5)
        (bind _returnvalue_6 (* _orbitaldistance 2500.0))
        (bind _returnvalue_7 (`|SpawnActorFromClass` "/Game/SGSG/Blueprints/Map/BP_Planet.BP_Planet_C" (`KismetMathLibrary.MakeTransform` (+ (`KismetMathLibrary.MakeVector` (* _returnvalue_6 (`KismetMathLibrary.Sin` _returnvalue_2)) (* _returnvalue_6 (`KismetMathLibrary.Cos` _returnvalue_2))) (`self.K2_GetActorLocation`)) (`KismetMathLibrary.MakeRotator` 0.0 0.0 (`KismetMathLibrary.RandomFloatInRange` 0.0 360.0))) "Undefined" "MultiplyWithRoot" null null))
        (bind _sphere (`/Game/SGSG/Blueprints/Map/BP_Planet.Sphere` _returnvalue_7))
        (bind _returnvalue_8 (/ (`KismetMathLibrary.Sqrt` _bodysize) 2.0))
        (`SceneComponent.SetRelativeScale3D` _sphere (`KismetMathLibrary.MakeVector` _returnvalue_8 _returnvalue_8 _returnvalue_8))
        (`/Game/SGSG/Blueprints/Map/BP_Planet.SetName` _returnvalue_7 _bodyname)
        (if (not (`|EnumEquality` _bodytype "NewEnumerator1"))
          (`PrimitiveComponent.SetMaterial` _sphere 0 (`BlueprintMapLibrary.Map_Find` (`self.PlanetTypeMap`) _bodytype))
          (`PrimitiveComponent.SetMaterial` _sphere 0 (`BlueprintMapLibrary.Map_Find` (`self.PlanetTypeMap`) _bodytype))
          (else
            (`PrimitiveComponent.SetMaterial` _sphere 0 (`BlueprintMapLibrary.Map_Find` (`self.RockyTypeMap`) _rockytype))))
        (`KismetArrayLibrary.Array_Add` (`self.Planets`) _returnvalue_7)
        (for _array_element_2 _moons
          (bind _returnvalue_9 (`self.K2_GetActorLocation` (`|GetArrayItem` (`self.Planets`) _array_index)))
          (bind (_bodyname_2 _orbitaldistance_2 _bodysize_2 _moontype _rockytype_2) (break `/Game/SGSG/Data/structs/S_MoonInfo` _array_element_2))
          (bind _returnvalue_10 (+ (* _orbitaldistance_2 50.0) 0.1))
          (bind _returnvalue_11 (`|SpawnActorFromClass` "/Script/Engine.StaticMeshActor" (`KismetMathLibrary.MakeTransform` _returnvalue_9 (struct) (`KismetMathLibrary.MakeVector` _returnvalue_10 _returnvalue_10 _returnvalue_10)) "Undefined" "MultiplyWithRoot" null null))
          (`StaticMeshActor.SetMobility` _returnvalue_11 "Stationary")
          (bind _staticmeshcomponent_2 (`StaticMeshActor.StaticMeshComponent` _returnvalue_11))
          (`StaticMeshComponent.SetStaticMesh` _staticmeshcomponent_2 "/Engine/BasicShapes/Plane.Plane")
          (`PrimitiveComponent.SetMaterial` _staticmeshcomponent_2 0 "/Game/SGSG/Materials/materials/M_Orbit.M_Orbit")
          (`PrimitiveComponent.SetCollisionProfileName` _staticmeshcomponent_2 "NoCollision" true)
          (`KismetArrayLibrary.Array_Add` (`self.Orbitals`) _returnvalue_11)
          (bind _returnvalue_12 (* _orbitaldistance_2 2500.0))
          (bind _returnvalue_13 (`|SpawnActorFromClass` "/Game/SGSG/Blueprints/Map/BP_Planet.BP_Planet_C" (`KismetMathLibrary.MakeTransform` (+ (`KismetMathLibrary.MakeVector` (* _returnvalue_12 (`KismetMathLibrary.Sin` _returnvalue)) (* _returnvalue_12 (`KismetMathLibrary.Cos` _returnvalue))) _returnvalue_9) (`KismetMathLibrary.MakeRotator` 0.0 0.0 (`KismetMathLibrary.RandomFloatInRange` 0.0 360.0))) "Undefined" "MultiplyWithRoot" null null))
          (bind _sphere_2 (`/Game/SGSG/Blueprints/Map/BP_Planet.Sphere` _returnvalue_13))
          (`PrimitiveComponent.SetMaterial` _sphere_2 0 (`BlueprintMapLibrary.Map_Find` (`self.RockyTypeMap`) _rockytype_2))
          (bind _returnvalue_14 (/ (`KismetMathLibrary.Sqrt` _bodysize_2) 2.0))
          (`SceneComponent.SetRelativeScale3D` _sphere_2 (`KismetMathLibrary.MakeVector` _returnvalue_14 _returnvalue_14 _returnvalue_14))
          (`/Game/SGSG/Blueprints/Map/BP_Planet.SetName` _returnvalue_13 _bodyname_2)
          (`KismetArrayLibrary.Array_Add` (`self.Moons`) _returnvalue_13))))))

(event `ClearSystem`
  (bind _orbitals (`self.Orbitals`))
  (bind _moons (`self.Moons`))
  (bind _planets (`self.Planets`))
  (for _array_element _planets
    (`self.K2_DestroyActor` _array_element))
  (`KismetArrayLibrary.Array_Clear` _planets)
  (for _array_element_2 _moons
    (`self.K2_DestroyActor` _array_element_2))
  (`KismetArrayLibrary.Array_Clear` _moons)
  (for _array_element_3 _orbitals
    (`self.K2_DestroyActor` _array_element_3))
  (`KismetArrayLibrary.Array_Clear` _orbitals))

(fn `UserConstructionScript`)